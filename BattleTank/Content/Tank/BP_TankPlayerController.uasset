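; BP_TankPlayerController is the tank player controller that shows the player UI, including the crosshair, and sets game input for the BattleGround level.
; It creates the BP_PlayerUI widget on BeginPlay, then checks the current level name every Tick.
; When the name is BattleGround, a DoOnce adds the widget to the viewport and calls GameStart, which switches player 0 to game-only input.
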(event `self.ReceiveBeginPlay`
  ;[1 1 1] Creation of Crosshair during GameMode
  (bind _returnvalue (`|CreateWidget` "/Game/UI/BP_PlayerUI.BP_PlayerUI_C")))

(event `self.ReceiveTick`
  (params (DeltaSeconds :type "Float (single-precision)"))
  ;[1 1 1] Creation of Crosshair during GameMode
  (bind _returnvalue (`GameplayStatics.GetCurrentLevelName` true))
  (if (`KismetStringLibrary.EqualEqual_StrStr` _returnvalue "BattleGround")
    (`/Engine/EditorBlueprintResources/StandardMacros.DoOnce` false
      (:`Completed`
        (`UserWidget.AddToViewport` (stale `self.ReceiveBeginPlay` _returnvalue) 0)
        (`self.GameStart`)))))

(event `GameStart`
  ;[1 1 1] Restore Input Commands for Game Mode
  (`WidgetBlueprintLibrary.SetInputMode_GameOnly` (`GameplayStatics.GetPlayerController` 0)))

(fn `UserConstructionScript`)